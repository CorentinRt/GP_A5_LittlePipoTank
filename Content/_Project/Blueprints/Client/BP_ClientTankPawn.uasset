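; Client-side tank pawn that supplies the audio and visual feedback for a tank in the game.
; It plays 2D sounds on spawn, on getting shot and on firing, with the firing sound picked randomly from an array.
; A material event recolors the body and head meshes after a validity check.
; Tank destruction spawns an explosion effect actor at the pawn's location, also triggerable through a debug event.
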(event Custom|CE_DebugPlayExplosionEffect
  ;[0.875 0.1929 0.6657 0.5] Receive On Tank Destroyed
  (Utilities|FlowControl|Sequence
    (:then_0
      (Game|SpawnActorfromClass "/Game/_Project/Blueprints/Client/Effects/BP_ExplosionEffect.BP_ExplosionEffect_C" (Math|Transform|MakeTransform (Transformation|GetActorLocation) "0, 0, 0" "1.000000,1.000000,1.000000") "AlwaysSpawn" "MultiplyWithRoot" 0 0))))

(event EventBeginPlay
  (Audio|PlaySound2D "/Game/_Project/Assets/Audio/Clip/Tank_Connexion.Tank_Connexion" 1.0 1.0 0.0 0 0))

(event Collision|EventActorBeginOverlap
  (params (OtherActor :type Actor%20Object%20Reference)))

(event EventTick
  (params (DeltaSeconds :type Float%20%28single-precision%29)))

(event EventGetShoot
  (Audio|PlaySound2D "/Game/_Project/Assets/Audio/Clip/Tank_Explosion.Tank_Explosion" 1.0 1.0 0.0 0 0))

(event EventShooting
  (Audio|PlaySound2D (Utilities|Array|Get(acopy) (Variables|Default|GetShootsSounds) (Math|Conversions|ToInteger(Byte) (Class|KismetMathLibrary|RandomInteger64inRange 0 (Class|KismetMathLibrary|ToInt64(Integer) (Utilities|Array|Length (Variables|Default|GetShootsSounds)))))) 1.0 1.0 0.0 0 0))

(event EventSetMeshMaterial
  (params (Material :type Material%20Interface%20Object%20Reference))
  (Utilities|IsValid Material
    (:Is%20Valid
      (Rendering|Material|SetMaterial (Variables|Default|GetTankBodyMesh) 0 Material)
      (Rendering|Material|SetMaterial (Variables|Default|GetTankHeadMesh) 0 Material))
    (:Is%20Not%20Valid
      (Development|PrintString "Can't set material to tank, material not valid." true true "(R=1.000000,G=0.074965,B=0.082604,A=1.000000)"))))

(event EventOnTankDestroy
  ;[0.875 0.1929 0.6657 0.5] Receive On Tank Destroyed
  (Utilities|FlowControl|Sequence
    (:then_0
      (Game|SpawnActorfromClass "/Game/_Project/Blueprints/Client/Effects/BP_ExplosionEffect.BP_ExplosionEffect_C" (Math|Transform|MakeTransform (Transformation|GetActorLocation) "0, 0, 0" "1.000000,1.000000,1.000000") "AlwaysSpawn" "MultiplyWithRoot" 0 0))))

(fn ConstructionScript)