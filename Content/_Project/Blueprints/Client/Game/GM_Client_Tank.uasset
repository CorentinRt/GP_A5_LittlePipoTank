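; Client game mode for the tank game that sets the main camera view and reacts to game phase changes.
; On BeginPlay it finds the first CameraActor tagged MainCamera and makes it the view target.
; Phase changes print the new phase, stop the music and swap between waiting-screen and in-game tracks.
; Debug events force phases (pre, in and post all set GAME) or start explosion camera shake; stopping it is a stub.
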(event Custom|CE_SetViewToMainCamera
  ;[0.2243 0.7865 0.7213 0.5] Set View To Main Camera
  (bind _maincamera (Variables|Default|GetMainCamera)
    (:then
      (Game|Player|SetViewTargetwithBlend (Game|GetPlayerController 0) _maincamera 0.0 "VTBlend_Linear" 0.0 false))
    (:else)))

(event Custom|CE_GetMainCamera
  ;[0.2451 0.8132 0.8531 0.5] Get Main Camera
  (bind _outactors (Actor|GetAllActorswithTag "MainCamera"))
  (bind _array_element (Utilities|Array|ForEachLoopwithBreak _outactors :!label _label)
    (:LoopBody
      (bind _ascamera_actor (Utilities|Casting|CastToCameraActor _array_element))
      (Variables|Default|SetMainCamera _ascamera_actor)
      (goto _label Break))))

(event Custom|CE_DebugPlayTankExplosionCameraShake
  (Game|Feedback|ClientStartCameraShake (Game|GetPlayerController 0) "/Game/_Project/Blueprints/Client/CameraShakes/BP_TankExplosionCameraShake.BP_TankExplosionCameraShake_C" 1.0 "CameraLocal" "0, 0, 0"))

(event Custom|CE_DebugForcePostGame
  ;[0.7552 0.04255 0.1585 0.5] Debug Force Set Phase
  (Class|GameModeTankClient|SetClientGamePhase "POST_GAME"))

(event Custom|CE_DebugForceWaitingGame
  ;[0.7552 0.04255 0.1585 0.5] Debug Force Set Phase
  (Class|GameModeTankClient|SetClientGamePhase "WAITING_PLAYER"))

(event Custom|CE_DebugForceInGame
  ;[0.7552 0.04255 0.1585 0.5] Debug Force Set Phase
  (Class|GameModeTankClient|SetClientGamePhase "IN_GAME"))

(event Custom|CE_DebugForcePreGame
  ;[0.7552 0.04255 0.1585 0.5] Debug Force Set Phase
  (Class|GameModeTankClient|SetClientGamePhase "PRE_GAME"))

(event Custom|CE_DebugStopTankExplosionCameraShake
  (Variables|Default|GetTankExplosionCameraShake
    (:then)
    (:else)))

(event EventReactChangeGamePhaseImplementation
  (params (InGamePhase :type ETankGamePhase%20Enum :default "WAITING_PLAYER"))
  (bind _main_game_music (Variables|Default|GetMain_Game_Music))
  ;[0.291 0.7477 0.874 0.5] React Change Game Phase
  (Development|PrintString (Utilities|String|Append "New Game Phase : " (Utilities|String|EnumtoString InGamePhase)))
  (switch Utilities|FlowControl|Switch|SwitchonETankGamePhase InGamePhase
    (:WAITING_PLAYER
      (Audio|Components|Audio|Stop _main_game_music)
      (Audio|Components|Audio|SetSound _main_game_music "/Game/_Project/Assets/Audio/Music/Waiting_Screen_Music.Waiting_Screen_Music"))
    (:IN_GAME
      (Audio|Components|Audio|Stop _main_game_music)
      (Audio|Components|Audio|SetSound _main_game_music "/Game/_Project/Assets/Audio/Music/Main_Game_Music.Main_Game_Music"))))

(event EventBeginPlay
  ;[0.1733 0.8385 0.2641 0.5] Begin Play
  (|CallParentFunction)
  (Utilities|FlowControl|Sequence
    (:then_0
      (CallFunction|CEGetMainCamera))
    (:then_1
      (CallFunction|CESetViewtoMainCamera))))

(fn ConstructionScript)