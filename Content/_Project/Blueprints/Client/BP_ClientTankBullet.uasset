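; Client-side tank bullet actor that provides the audiovisual feedback for a projectile.
; On BeginPlay it spawns shoot effects and plays the fire sound at its location, a sequence a debug event can replay.
; Bounce events play a sound, throttled by a DoOnce that resets after a short delay.
; Destruction triggers a custom event that plays the destroyed sound.
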(event Custom|CE_DebugPlayShootEffect
  ;[0.3671 0.8281 0.3258 0.5] Begin Play
  (Utilities|FlowControl|Sequence
    (:then_0
      (Game|SpawnActorfromClass "/Game/_Project/Blueprints/Client/Effects/BP_ShootEffects.BP_ShootEffects_C" (Math|Transform|MakeTransform (Transformation|GetActorLocation) "0, 0, 0" "1.000000,1.000000,1.000000") "AlwaysSpawn" "MultiplyWithRoot" 0 0))
    (:then_1
      (Audio|PlaySoundatLocation "/Game/_Project/Assets/Audio/SFX/Bullets/MS_FireBullet.MS_FireBullet" (Transformation|GetActorLocation) "0, 0, 0" 1.0 1.0 0.0 0 0 0 0))))

(event Custom|CE_PlayOnDestroyedEffect
  ;[0.9167 0.2226 0.874 0.5] CE_On Destroyed Effect
  (Utilities|FlowControl|Sequence
    (:then_0
      (Audio|PlaySoundatLocation "/Game/_Project/Assets/Audio/SFX/Bullets/MS_DestroyedBullet.MS_DestroyedBullet" (Transformation|GetActorLocation) "0, 0, 0" 1.0 1.0 0.0 0 0 0 0))))

(event EventOnBulletBounced
  ;[0.8594 0.2545 0.7564 0.5] Receive On bullet bounced
  (Utilities|FlowControl|Sequence
    (:then_0
      (Utilities|FlowControl|DoOnce false :!label _label
        (:Completed
          (Audio|PlaySoundatLocation "/Game/_Project/Assets/Audio/SFX/Bullets/MS_BounceBullet.MS_BounceBullet" (Transformation|GetActorLocation) "0, 0, 0" 1.0 1.0 0.0 0 0 0 0)
          (Utilities|FlowControl|Delay 1.0)
          (goto _label Reset))))))

(event EventDestroyed
  ;[0.8698 0.1115 0 0.5] Destroyed
  (Utilities|FlowControl|Sequence
    (:then_0
      (CallFunction|CEPlayonDestroyedEffect))))

(event EventBeginPlay
  ;[0.3671 0.8281 0.3258 0.5] Begin Play
  (Utilities|FlowControl|Sequence
    (:then_0
      (Game|SpawnActorfromClass "/Game/_Project/Blueprints/Client/Effects/BP_ShootEffects.BP_ShootEffects_C" (Math|Transform|MakeTransform (Transformation|GetActorLocation) "0, 0, 0" "1.000000,1.000000,1.000000") "AlwaysSpawn" "MultiplyWithRoot" 0 0))
    (:then_1
      (Audio|PlaySoundatLocation "/Game/_Project/Assets/Audio/SFX/Bullets/MS_FireBullet.MS_FireBullet" (Transformation|GetActorLocation) "0, 0, 0" 1.0 1.0 0.0 0 0 0 0))))

(fn ConstructionScript)