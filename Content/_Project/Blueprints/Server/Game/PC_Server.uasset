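; PC_Server is a server-side player controller, going by its name, that puts the view on the level's main camera at startup.
; On BeginPlay it finds actors tagged MainCamera and stores the first one that casts to CameraActor.
; It then sets that camera as the view target of player controller 0, looked up by index, if the reference is valid.
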(event Custom|CE_SetViewToMainCamera
  ;[0.2243 0.7865 0.7213 0.5] Set View To Main Camera
  (bind _maincamera (Variables|Default|GetMainCamera)
    (:then
      (Game|Player|SetViewTargetwithBlend (Game|GetPlayerController 0) _maincamera 0.0 "VTBlend_Linear" 0.0 false))
    (:else)))

(event Custom|CE_GetMainCamera
  ;[0.2451 0.8132 0.8531 0.5] Get Main Camera
  (bind _outactors (Actor|GetAllActorswithTag "MainCamera"))
  (bind _array_element (Utilities|Array|ForEachLoopwithBreak _outactors :!label _label)
    (:LoopBody
      (bind _ascamera_actor (Utilities|Casting|CastToCameraActor _array_element))
      (Variables|Default|SetMainCamera _ascamera_actor)
      (goto _label Break))))

(event EventBeginPlay
  ;[0.2592 0.8031 0.1213 0.5] Begin Play
  (Utilities|FlowControl|Sequence
    (:then_0
      (CallFunction|CEGetMainCamera))
    (:then_1
      (CallFunction|CESetViewtoMainCamera))))

(fn ConstructionScript)